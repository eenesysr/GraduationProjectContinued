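; Right-hand door actor that swings open and closed when its Interact event fires.
; A FlipFlop alternates playing and reversing a timeline, which lerps the static mesh's relative yaw between two angles.
; Each timeline update sets IsActives unless the actor's yaw exactly equals an end angle, and Interact is ignored while that flag is set.
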(event EventInteract
  (bind _self self)
  (bind _returnvalue (Transformation|GetActorRotation _self))
  (if (not (Variables|Default|Getis%20Actives))
    (Utilities|FlowControl|FlipFlop
      (:A
        (bind _door_timeline (Timeline|Timeline Play)
          (:Update
            (Transformation|SetRelativeRotation (Variables|Debug|GetStaticMeshComponent) (Math|Rotator|MakeRotator 0.0 0.0 (Math|Float|Lerp 1.8e+02 2.8e+02 _door_timeline)) false false)
            (if (or (== (.yaw _returnvalue) 1.8e+02) (or (== (.yaw _returnvalue) 2.8e+02) (== (.yaw _returnvalue) -8e+01)))
              (Variables|Default|Setis%20Actives false)
              (else
                (Variables|Default|Setis%20Actives true))))))
      (:B
        (Timeline|Timeline Reverse)))))

(fn ConstructionScript)