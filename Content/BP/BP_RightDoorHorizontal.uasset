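; BP_RightDoorHorizontal is a door Blueprint that swings its static mesh open and closed when its Interact event fires.
; A FlipFlop alternates between playing and reversing a Timeline, which lerps the mesh's relative yaw between 90 and 190 degrees.
; Each update sets IsActives, which blocks further interaction, unless the actor's yaw, rather than the mesh's, exactly matches an end angle.
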(event EventInteract
  (bind _self self)
  (bind _returnvalue (Transformation|GetActorRotation _self))
  (if (not (Variables|Default|Getis%20Actives))
    (Utilities|FlowControl|FlipFlop
      (:A
        (bind _door_timeline (Timeline|Timeline Play)
          (:Update
            (Transformation|SetRelativeRotation (Variables|Debug|GetStaticMeshComponent) (Math|Rotator|MakeRotator 0.0 0.0 (Math|Float|Lerp 9e+01 1.9e+02 _door_timeline)) false false)
            (if (or (== (.yaw _returnvalue) 9e+01) (or (== (.yaw _returnvalue) 1.9e+02) (== (.yaw _returnvalue) -1.7e+02)))
              (Variables|Default|Setis%20Actives false)
              (else
                (Variables|Default|Setis%20Actives true))))))
      (:B
        (Timeline|Timeline Reverse)))))

(fn ConstructionScript)