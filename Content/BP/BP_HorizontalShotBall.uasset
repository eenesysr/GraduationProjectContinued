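; BP_HorizontalShotBall is an interactable physics ball that fires horizontally and then resets itself.
; On Interact it stores its location, pushes its mesh along world X with an impulse, then after a short delay destroys itself and spawns a fresh copy at that spot.
; Disconnected leftovers hold a timeline-driven movement toggle and math expressions for computing horizontal-throw distance from height, gravity and speed.
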(event EventInteract
  (Variables|Default|SetOriginalLocation (Transformation|GetActorLocation self))
  (Physics|AddImpulse (Variables|Debug|GetStaticMeshComponent) "50.000000,0.000000,0.000000" "None" false)
  (Utilities|FlowControl|Delay 2.0)
  (Actor|DestroyActor self)
  (Game|SpawnActorfromClass "BP_HorizontalShotBall_C" (Math|Transform|MakeTransform (Variables|Default|GetOriginalLocation) "0, 0, 0" "1.000000,1.000000,1.000000") "Undefined" "MultiplyWithRoot" 0 0))

(fn ConstructionScript)