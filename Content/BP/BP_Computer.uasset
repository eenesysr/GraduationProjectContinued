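; BP_Computer is an interactable computer that moves the player's view to itself and hands input to its widget.
; A box overlap with BP_FirstPersonCharacter toggles CanLookComputer, which gates a debug E key on the actor's own enabled input.
; Pressing it blends the view target to the computer, sets UI-only input focused on the widget, then hides the mouse cursor after the blend-length delay.
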(event OnComponentBeginOverlap(Box)
  (params (OverlappedComponent :type Primitive%20Component%20Object%20Reference) (OtherActor :type Actor%20Object%20Reference) (OtherComp :type Primitive%20Component%20Object%20Reference) (OtherBodyIndex :type Integer) (bFromSweep :type Boolean) (SweepResult :type Hit%20Result%20Structure%20%28by%20ref%29))
  (Utilities|Casting|CastToBP_FirstPersonCharacter OtherActor)
  (Variables|Default|SetbCanLookComputer true))

(event OnComponentEndOverlap(Box)
  (params (OverlappedComponent :type Primitive%20Component%20Object%20Reference) (OtherActor :type Actor%20Object%20Reference) (OtherComp :type Primitive%20Component%20Object%20Reference) (OtherBodyIndex :type Integer))
  (Utilities|Casting|CastToBP_FirstPersonCharacter OtherActor)
  (Variables|Default|SetbCanLookComputer false))

(event EventBeginPlay
  (Input|EnableInput (Game|GetPlayerController 0)))

(event Input|KeyboardEvents|DebugKeyE
  (params (Key :type Key%20Structure) (ActionValue :type Input%20Action%20Value%20Structure))
  (bind _returnvalue (Game|GetPlayerController 0))
  (:Pressed
    (if (Variables|Default|GetbCanLookComputer)
      (Game|Player|SetViewTargetwithBlend _returnvalue self 0.4 "VTBlend_Linear" 0.0 false)
      (Input|SetInputModeUIOnly _returnvalue (UserInterface|GetWidget (Variables|Default|GetWidget)) "DoNotLock" false)
      (Utilities|FlowControl|Delay 0.4)
      (Variables|/Script/Engine.PlayerController|SetbShowMouseCursor _returnvalue false))))

(fn ConstructionScript)